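; BP_Collection_Component handles coin and puzzle piece pickups and their HUD feedback.
; On BeginPlay it creates both counter widgets hidden.
; CollectCoin adds to the total, updates and shows the counter, and starts a looping timer that clears a recent-collection flag, then hides the widget on a later tick.
; CollectPuzzlePiece sets three flags by comparing the piece number and shows its widget briefly using a Delay.
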(event Custom|Hide%20Coin%20Counter
  ;[1 1 1] Coin Timer Removal
  (if (Variables|Default|GetrecentCollection)
    (bind _index (Utilities|FlowControl|ForLoopwithBreak 0 (Variables|Default|GethideDelay) :!label _label)
      (:LoopBody
        (if (>= (Variables|Default|GethideDelay) _index)
          (Variables|Default|SetrecentCollection false)
          (else
            (Math|Integer|IncrementInt _index)))))
    (else
      (Utilities|FlowControl|Sequence
        (:then_0
          (goto _label Break))
        (:then_1
          (Widget|SetVisibility (Variables|Default|GetCoinCounterREF) "Hidden")
          (Utilities|Time|ClearandInvalidateTimerbyHandle (Variables|Default|GetTE_CoinCounterHandle)))))))

(event EventCollectPuzzlePiece
  (params (Which%20Is%20Colleceted :type Integer))
  ;[1 1 1] Is Puzzle Piece Collected
  (if (not (== Which%20Is%20Colleceted 0))
    ;[1 1 1] Show Puzzle Piece Collected
    (Widget|SetVisibility (Variables|Default|GetPuzzlePieceREF) "Visible")
    ;[1 1 1] Which Puzzle Piece is Collected
    (Variables|Default|Set1_Is_Collected (== Which%20Is%20Colleceted 1))
    (Variables|Default|Set2_Is_Collected (== Which%20Is%20Colleceted 2))
    (Variables|Default|Set3_Is_Collected (== Which%20Is%20Colleceted 3))
    ;[1 1 1] Re-Hide Widget
    (Utilities|FlowControl|Delay 3.0)
    (Widget|SetVisibility (Variables|Default|GetPuzzlePieceREF) "Hidden")))

(event EventCollectCoin
  (params (Value :type Integer))
  ;[1 1 1] Is Coin Collected
  (if (not (== Value 0))
    ;[1 1 1] Show Coin Counter
    (Variables|Default|SetrecentCollection true)
    (Widget|SetVisibility (Variables|Default|GetCoinCounterREF) "Visible")
    ;[1 1 1] Increase Coin Counter by One
    (bind _output_get (Variables|Default|SetTotal%20Coins (+ Value (Variables|Default|GetTotal%20Coins))))
    (Rendering|Components|TextRender|SetText (Variables|/Game/ColletionStuff/Collectables/Coin/WBP_Coin_Counter.WBP_Coin_Counter_C|GetCoinTotal (Variables|Default|GetCoinCounterREF)) (Utilities|Text|ToText(Integer) _output_get))
    ;[1 1 1] Create Event and Reference Handle
    (bind _returnvalue (Utilities|Time|SetTimerbyEvent (delegate Custom|Hide%20Coin%20Counter) 1.0 true))
    (Variables|Default|SetTE_CoinCounterHandle _returnvalue)))

(event EventBeginPlay
  ;[1 1 1] Create Widget / Hide on BeginPlay
  (Utilities|FlowControl|Sequence
    (:then_0
      ;;[1 1 1] Coin Widget
      (bind _returnvalue (UserInterface|CreateWidget "/Game/ColletionStuff/Collectables/Coin/WBP_Coin_Counter.WBP_Coin_Counter_C"))
      (bind _output_get (Variables|Default|SetCoinCounterREF _returnvalue))
      (UserInterface|Viewport|AddtoViewport _output_get 0)
      (Widget|SetVisibility _output_get "Hidden"))
    (:then_1
      ;;[1 1 1] Puzzle Piece Widget
      (bind _returnvalue_2 (UserInterface|CreateWidget "/Game/ColletionStuff/Collectables/PuzzlePiece/WBP_PuzzlePiece.WBP_PuzzlePiece_C"))
      (bind _output_get_2 (Variables|Default|SetPuzzlePieceREF _returnvalue_2))
      (UserInterface|Viewport|AddtoViewport _output_get_2 0)
      (Widget|SetVisibility _output_get_2 "Hidden"))))

(event EventTick
  (params (DeltaSeconds :type Float%20%28single-precision%29))
  ;[1 1 1] Create Widget / Hide on BeginPlay
  ;;[1 1 1] Is Working?
)