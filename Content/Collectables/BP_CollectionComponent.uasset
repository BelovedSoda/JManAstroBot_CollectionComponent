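; Collection component that records coin, puzzle piece and friend pickups and briefly shows a HUD widget for each.
; BeginPlay creates the three widgets hidden.
; Puzzle and friend events set three flags by comparing the incoming ID, overwriting earlier values, then hide their widget after a fixed Delay.
; Coin pickups update the total and start a looping timer that clears a recent-collection flag, then hides the counter on a later firing.
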(event Custom|Hide%20Coin%20Counter
  (bind _hidedelay (Variables|Default|GetHideDelay))
  (if (Variables|Default|GetRecentCollection)
    (bind _index (Utilities|FlowControl|ForLoopwithBreak 0 _hidedelay :!label _label)
      (:LoopBody
        (if (>= _hidedelay _index)
          (Variables|Default|SetRecentCollection false)
          (else
            (Math|Integer|IncrementInt _index)))))
    (else
      (Utilities|FlowControl|Sequence
        (:then_0
          (goto _label Break))
        (:then_1
          (Widget|SetVisibility (Variables|Default|GetCoinCounterREF) "Hidden")
          (Utilities|Time|ClearandInvalidateTimerbyHandle (Variables|Default|GetTE%20Coin%20Counter%20Handle)))))))

(event EventBeginPlay
  ;[1 1 1] Create Widget/Hide on BeginPlay
  (Utilities|FlowControl|Sequence
    (:then_0
      ;;[1 1 1] CoinWidget
      (bind _returnvalue (UserInterface|CreateWidget "/JManAstroBot_ColectionComp/Collectables/Coin/WBP_CoinCounter.WBP_CoinCounter_C"))
      (bind _output_get (Variables|Default|SetCoinCounterREF _returnvalue))
      (UserInterface|Viewport|AddtoViewport _output_get 0)
      (Widget|SetVisibility _output_get "Hidden"))
    (:then_1
      ;;[1 1 1] PuzzlePieceWidget
      (bind _returnvalue_2 (UserInterface|CreateWidget "/JManAstroBot_ColectionComp/Collectables/PuzzlePiece/WBP_PuzzlePiece.WBP_PuzzlePiece_C"))
      (bind _output_get_2 (Variables|Default|SetPuzzlePieceREF _returnvalue_2))
      (UserInterface|Viewport|AddtoViewport _output_get_2 0)
      (Widget|SetVisibility _output_get_2 "Hidden"))
    (:then_2
      ;;[1 1 1] FriendWidget
      (bind _returnvalue_3 (UserInterface|CreateWidget "/JManAstroBot_ColectionComp/Collectables/Character/WBP_Friends.WBP_Friends_C"))
      (bind _output_get_3 (Variables|Default|SetFriends%20REF _returnvalue_3))
      (UserInterface|Viewport|AddtoViewport _output_get_3 0)
      (Widget|SetVisibility _output_get_3 "Hidden"))))

(event EventTick
  (params (DeltaSeconds :type Float%20%28single-precision%29))
  ;[1 1 1] Create Widget/Hide on BeginPlay
)

(event EventCollectPuzzlePiece
  (params (Which%20Is%20Collected :type Integer))
  (if (not (== Which%20Is%20Collected 0))
    (Widget|SetVisibility (Variables|Default|GetPuzzlePieceREF) "Visible")
    (Variables|Default|Set1IsCollected (== Which%20Is%20Collected 1))
    (Variables|Default|Set2IsCollected (== Which%20Is%20Collected 2))
    (Variables|Default|Set3IsCollected (== Which%20Is%20Collected 3))
    (Utilities|FlowControl|Delay 3.0)
    (Widget|SetVisibility (Variables|Default|GetPuzzlePieceREF) "Hidden")))

(event EventCollectCoin
  (params (Value :type Integer))
  (if (not (== Value 0))
    (Variables|Default|SetRecentCollection true)
    (Widget|SetVisibility (Variables|Default|GetCoinCounterREF) "Visible")
    (bind _output_get (Variables|Default|SetTotalCoins (+ Value (Variables|Default|GetTotalCoins))))
    (Rendering|Components|TextRender|SetText (Variables|/JManAstroBot_ColectionComp/Collectables/Coin/WBP_CoinCounter.WBP_CoinCounter_C|GetCoinTotal (Variables|Default|GetCoinCounterREF)) (Utilities|Text|ToText(Integer) _output_get))
    (bind _returnvalue (Utilities|Time|SetTimerbyEvent (delegate Custom|Hide%20Coin%20Counter) 1.0 true))
    (Variables|Default|SetTE%20Coin%20Counter%20Handle _returnvalue)))

(event EventCollectFriend
  (params (Which%20Friend :type Integer))
  (if (not (== Which%20Friend 0))
    (Widget|SetVisibility (Variables|Default|GetFriends%20REF) "Visible")
    (Variables|Default|SetFriend1Collected (== Which%20Friend 1))
    (Variables|Default|SetFriend2Collected (== Which%20Friend 2))
    (Variables|Default|SetFriend3Collected (== Which%20Friend 3))
    (Utilities|FlowControl|Delay 3.0)
    (Widget|SetVisibility (Variables|Default|GetFriends%20REF) "Hidden")))