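; Template collectable actor that is either a friend freed by punching or a pickup collected on touch, selected by the Friend flag.
; Friends react to PunchActor once, reporting FriendNum to a component on player character 0 before destroying themselves.
; Other pickups use sphere overlap to find that component on the overlapping actor, send both coin value and puzzle piece number, play a coin sound and destroy themselves.
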(event OnComponentBeginOverlap(Sphere)
  (params (OverlappedComponent :type Primitive%20Component%20Object%20Reference) (OtherActor :type Actor%20Object%20Reference) (OtherComp :type Primitive%20Component%20Object%20Reference) (OtherBodyIndex :type Integer) (bFromSweep :type Boolean) (SweepResult :type Hit%20Result%20Structure%20%28by%20ref%29))
  (bind _compoentclassref (Variables|Default|GetCompoentClassREF))
  (bind _returnvalue (Actor|GetComponentbyClass OtherActor _compoentclassref))
  (if (not (Variables|Default|GetFriend?))
    (Utilities|IsValid _returnvalue
      (:Is%20Valid
        (Class|BPICollection|CollectCoin(Message) _returnvalue (Variables|Default|GetCoinValue))
        (Class|BPICollection|CollectPuzzlePiece(Message) _returnvalue (Variables|Default|GetPuzzlePieceNum))
        (Audio|PlaySoundatLocation "/JManAstroBot_ColectionComp/Collectables/402067__matrixxx__retro-coin-01.402067__matrixxx__retro-coin-01" (Transformation|GetWorldLocation (Variables|Default|GetColectableDefault)) "0, 0, 0" 1.0 1.0 0.0 0 0 0 0)
        (Actor|DestroyActor)))))

(event EventPunchActor
  (params (Damage :type Float%20%28double-precision%29) (Force%20Location :type Vector :default "0, 0, 0") (Punch%20Type :type E_PunchTypes%20Enum :default "NewEnumerator0"))
  ;[1 1 1] Punch Friend
  (if (Variables|Default|GetFriend?)
    (Utilities|FlowControl|DoOnce false
      (:Completed
        (Class|BPICollection|CollectFriend(Message) (Actor|GetComponentbyClass (Game|GetPlayerCharacter 0) (Variables|Default|GetCompoentClassREF)) (Variables|Default|GetFriendNum))
        (Actor|DestroyActor)))))

(fn ConstructionScript)